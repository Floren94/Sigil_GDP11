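; Base enemy Blueprint that wires up an overhead health bar and handles death with a dissolve effect.
; BeginPlay binds the GAS health attribute set to the widget and a change handler, creates dynamic mesh materials and async-loads the dissolve Niagara system.
; At zero health it hides the bar, attaches the FX sampling the skeletal mesh, activates Status.Dead abilities and runs a timeline driving material dissolve before destroying the actor.
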(event `self.ReceiveBeginPlay`
  (bind _mesh (`self.Mesh`))
  (bind _mesh_2 (`self.Mesh`))
  (`|ExecutionSequence`
    (:`then_0`
      (bind _aswbp_health_bar_enemy (cast `/Game/Sigil/Characters/Enemies/UI/WBP_HealthBarEnemy` (`WidgetComponent.GetUserWidgetObject` (`self.Widget`))))
      (bind _returnvalue (`AbilitySystemComponent.GetAttributeSet` (`AbilitySystemBlueprintLibrary.GetAbilitySystemComponent` null) "/Script/Sigil.SigilHealthAttributeSet"))
      (`/Game/Sigil/Characters/Enemies/UI/WBP_HealthBarEnemy.SetHealthAttributeSet` _aswbp_health_bar_enemy _returnvalue)
      (add `SigilHealthAttributeSet.OnHealthChanged` _returnvalue (delegate `OnHealthChanged_Event`)))
    (:`then_1`
      (`|ExecutionSequence`
        (:`then_0`
          (bind _returnvalue_2 (`PrimitiveComponent.CreateDynamicMaterialInstance` _mesh 0 (`PrimitiveComponent.GetMaterial` _mesh 0) "None"))
          (bind _output_get (set `self.Material1` _returnvalue_2))
          (`PrimitiveComponent.SetMaterial` _mesh_2 0 _output_get))
        (:`then_1`
          (bind _returnvalue_3 (`PrimitiveComponent.CreateDynamicMaterialInstance` _mesh 0 (`PrimitiveComponent.GetMaterial` _mesh 1) "None"))
          (bind _output_get_2 (set `self.Material2` _returnvalue_3))
          (`PrimitiveComponent.SetMaterial` _mesh_2 1 _output_get_2)
          (bind _object (`|LoadAsset` (`self.FXDissolveSoft`))
            (:`Completed`
              (bind _asniagara_system (cast `NiagaraSystem` _object))
              (set `self.FXDissolve` _asniagara_system))))))))

(event `OnHealthChanged_Event`
  (params (AttributeSet :type "AttributeSet Object Reference") (OldValue :type "Float (single-precision)") (NewValue :type "Float (single-precision)"))
  (if (<= NewValue 0.0)
    (`SceneComponent.SetVisibility` (`self.Widget`) false false)
    (bind _returnvalue (`NiagaraFunctionLibrary.SpawnSystemAttached` (`self.FXDissolve`) (`self.Mesh`) "None" (0.0 0.0 0.0) (struct) "SnapToTarget" true true "AutoRelease"))
    (bind _output_get (set `self.SpawnedFX` _returnvalue))
    (`NiagaraFunctionLibrary.OverrideSystemUserVariableSkeletalMeshComponent` _output_get "" (`self.Mesh`))
    (`AbilitySystemComponent.TryActivateAbilitiesByTag` (`self.GetSigilAbilityComponent`) (`BlueprintGameplayTagLibrary.MakeGameplayTagContainerFromTag` (struct :`TagName` "Status.Dead")) false)
    (bind (_direction _dissolveamount) (`Timeline|DeadTimeline` :!via `PlayFromStart`)
      (:`Update`
        (`|ExecutionSequence`
          (:`then_0`
            (`MaterialInstanceDynamic.SetScalarParameterValue` (`self.Material1`) "DissolveIntensity" _dissolveamount))
          (:`then_1`
            (`MaterialInstanceDynamic.SetScalarParameterValue` (`self.Material2`) "DissolveIntensity" _dissolveamount))))
      (:`Finished`
        (`self.K2_DestroyActor`)))))

(fn `UserConstructionScript`)