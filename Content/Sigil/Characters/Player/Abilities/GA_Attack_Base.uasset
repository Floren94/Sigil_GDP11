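; Base melee-style attack Gameplay Ability for the player that plays combo montages on the ground and a single montage in the air.
; A Grounded tag check selects either the montage at the combo counter in the Attacks map, with root motion translation zeroed, or the air attack.
; Any grounded montage exit advances the counter, resetting it after the last attack or through a short timer, then ends the ability.
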(event `self.K2_ActivateAbility`
  (`self.K2_CommitAbility`)
  (if (`GameplayTagAssetInterface.HasMatchingGameplayTag` (`AbilitySystemBlueprintLibrary.GetAbilitySystemComponent` (`self.GetPlayerCharacterFromInfo`)) (struct :`TagName` "Ability.Movement.Grounded"))
    (`AbilityTask_PlayMontageAndWait.CreatePlayMontageAndWaitProxy` "None" (`BlueprintMapLibrary.Map_Find` (`self.Attacks`) (`self.Counter`)) 1.0 "None" true 0.0
      (:`OnCompleted`
        _)
      (:`OnBlendOut`
        _)
      (:`OnInterrupted`
        _)
      (:`OnCancelled`
        _))
    (bind _result (`/Engine/EditorBlueprintResources/StandardMacros.IncrementInt` (`self.Counter`))
      (:`  `
        (if (>= _result (`BlueprintMapLibrary.Map_Length` (`self.Attacks`)))
          (`self.ResetCombo`)
          (else
            (`KismetSystemLibrary.K2_SetTimerDelegate` (delegate `ResetCombo`) 1.0)))
        (`self.K2_EndAbility`)))
    (else
      (`AbilityTask_PlayMontageAndWait.CreatePlayMontageAndWaitProxy` "None" "/Game/Sigil/Characters/Player/Animations/MageAnimPack/AM_AirAtt.AM_AirAtt"
        (:`OnCompleted`
          _)
        (:`OnBlendOut`
          _)
        (:`OnInterrupted`
          _)
        (:`OnCancelled`
          _))
      (`self.K2_EndAbility`))))

(event `ResetCombo`
  (set `self.Counter` 0))