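; Gameplay ability that toggles the player's staff weapon between equipped and unequipped.
; On activation it checks for the staff weapon tag on the ability system, removes or adds it on the player character, and plays the matching montage.
; A gameplay event fired during the montage tells the ItemAbilityComponent to equip or unequip the item.
; The ability ends when the montage completes, is interrupted or is cancelled.
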(event `self.K2_ActivateAbility`
  (`self.K2_CommitAbility`)
  (if (`GameplayTagAssetInterface.HasMatchingGameplayTag` (`self.GetAbilitySystemComponentFromActorInfo`) (struct :`TagName` "Ability.Player.Weapon.Staff"))
    (`SigilPlayerCharacter.RemoveGameplayTag` (`self.GetPlayerCharacterFromInfo`) (`BlueprintGameplayTagLibrary.MakeLiteralGameplayTag` (struct :`TagName` "Ability.Player.Weapon.Staff")))
    (`AbilityTask_PlayMontageAndWait.CreatePlayMontageAndWaitProxy` "None" "/Game/Sigil/Characters/Player/ABP/AM_UnEquip.AM_UnEquip"
      (:`then`
        (`AbilityTask_WaitGameplayEvent.WaitGameplayEvent` (struct :`TagName` "Ability.Player.Event.Unequip.Staff") null
          (:`EventReceived`
            (`ItemAbilityManagerComp.UnEquipItem` (`SigilCharacterBase.GetItemAbilityComponent` (`self.GetPlayerCharacterFromInfo`))))))
      (:`OnCompleted`
        (`self.K2_EndAbility` :!label _label))
      (:`OnInterrupted`
        (goto _label))
      (:`OnCancelled`
        (goto _label)))
    (else
      (`SigilPlayerCharacter.AddGameplayTag` (`self.GetPlayerCharacterFromInfo`) (`BlueprintGameplayTagLibrary.MakeLiteralGameplayTag` (struct :`TagName` "Ability.Player.Weapon.Staff")))
      (`AbilityTask_PlayMontageAndWait.CreatePlayMontageAndWaitProxy` "None" "/Game/Sigil/Characters/Player/ABP/AM_Equip.AM_Equip"
        (:`then`
          (`AbilityTask_WaitGameplayEvent.WaitGameplayEvent` (struct :`TagName` "Ability.Player.Event.Equip.Staff") null
            (:`EventReceived`
              (`ItemAbilityManagerComp.EquipItem` (`SigilCharacterBase.GetItemAbilityComponent` (`self.GetPlayerCharacterFromInfo`)) (struct :`TagName` "Ability.Player.Weapon.Staff")))))
        (:`OnCompleted`
          (`self.K2_EndAbility` :!label _label_2))
        (:`OnInterrupted`
          (goto _label_2))
        (:`OnCancelled`
          (goto _label_2))))))