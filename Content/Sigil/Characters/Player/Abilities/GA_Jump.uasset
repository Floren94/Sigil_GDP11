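; Player gameplay ability that performs the jump and the double jump.
; It ends at once if the DoubleJump tag is present; otherwise it commits and calls Jump.
; When the jump count is at least one, it adds that tag, an additive upward launch and a slowed montage, with a BlockMontage tag held until the montage finishes or is interrupted.
; The DoubleJump tag is not removed here.
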(event `self.K2_ActivateAbility`
  (if (`GameplayTagAssetInterface.HasMatchingGameplayTag` (`self.GetAbilitySystemComponentFromActorInfo`) (struct :`TagName` "Ability.Movement.DoubleJump"))
    (`self.K2_EndAbility`)
    (else
      (set `self.PlayerCharacter` (`self.GetPlayerCharacterFromInfo`))
      (`self.K2_CommitAbility`)
      (`Character.Jump` (`self.GetPlayerCharacterFromInfo`))
      (if (>= (`Character.JumpCurrentCount` (`self.PlayerCharacter`)) 1)
        (`SigilPlayerCharacter.AddGameplayTag` (`self.PlayerCharacter`) (`BlueprintGameplayTagLibrary.MakeLiteralGameplayTag` (struct :`TagName` "Ability.Movement.DoubleJump")))
        (`Character.LaunchCharacter` (`self.PlayerCharacter`) (0.0 0.0 800.0) false false)
        (`SigilPlayerCharacter.AddGameplayTag` (`self.PlayerCharacter`) (`BlueprintGameplayTagLibrary.MakeLiteralGameplayTag` (struct :`TagName` "Ability.BlockMontage")))
        (`AbilityTask_PlayMontageAndWait.CreatePlayMontageAndWaitProxy` "None" "/Game/Sigil/Characters/Player/ABP/AM_DoubleJump.AM_DoubleJump" 0.7
          (:`OnCompleted`
            _)
          (:`OnBlendOut`
            _)
          (:`OnInterrupted`
            _)
          (:`OnCancelled`
            _))
        (`SigilPlayerCharacter.RemoveGameplayTag` (`self.PlayerCharacter`) (`BlueprintGameplayTagLibrary.MakeLiteralGameplayTag` (struct :`TagName` "Ability.BlockMontage")))
        (`self.K2_EndAbility`)
        (else
          (`self.K2_EndAbility`))))))