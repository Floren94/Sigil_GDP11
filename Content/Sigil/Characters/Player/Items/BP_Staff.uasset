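; BP_Staff is the player's staff weapon, dealing GAS damage to other actors its collision overlaps during a light staff attack.
; A hit requires an open HitWindow, the owner's light-attack tag and a target implementing AbilitySystemInterface.
; The target's ASC creates and self-applies GE_DamageHealth using BaseDamage, then receives a HitReact event with player 0 as instigator.
; HitWindow closes on each hit and reopens after a short delay, throttling repeat hits.
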(event `self.ItemCollision.OnComponentBeginOverlap`
  (params (OverlappedComponent :type "PrimitiveComponent Object Reference") (OtherActor :type "Actor Object Reference") (OtherComp :type "PrimitiveComponent Object Reference") (OtherBodyIndex :type Integer) (bFromSweep :type Boolean) (SweepResult :type "HitResult Structure (by ref)"))
  (bind _returnvalue (`self.GetOwner`))
  (bind _returnvalue_2 (`self.GetComponentByClass` OtherActor "/Script/GameplayAbilities.AbilitySystemComponent"))
  (if (and (!= OtherActor _returnvalue) (`KismetSystemLibrary.DoesImplementInterface` OtherActor "/Script/GameplayAbilities.AbilitySystemInterface") (`self.HitWindow`) (`GameplayTagAssetInterface.HasMatchingGameplayTag` (`AbilitySystemBlueprintLibrary.GetAbilitySystemComponent` _returnvalue) (struct :`TagName` "Ability.Player.Attack.Light.Staff")))
    (set `self.HitWindow` false)
    (bind _returnvalue_3 (`AbilitySystemBlueprintLibrary.AssignTagSetByCallerMagnitude` (`AbilitySystemComponent.MakeOutgoingSpec` :`self` _returnvalue_2 :`GameplayEffectClass` "/Game/Sigil/Characters/Player/Abilities/G_Effects/GE_DamageHealth.GE_DamageHealth_C") (struct :`TagName` "Status.Damage") (`self.BaseDamage`)))
    (`AbilitySystemComponent.BP_ApplyGameplayEffectSpecToSelf` _returnvalue_2 _returnvalue_3)
    (`AbilitySystemBlueprintLibrary.SendGameplayEventToActor` OtherActor (struct :`TagName` "Ability.HitReact") (make `GameplayEventData` (struct) (`GameplayStatics.GetPlayerCharacter` 0)))
    (`KismetSystemLibrary.Delay` 0.5)
    (set `self.HitWindow` true)))

(fn `UserConstructionScript`)